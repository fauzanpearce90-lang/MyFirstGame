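; BP_myblueprint is a small Blueprint that tests player damage by reducing a HealthPoint variable, apparently as a function experiment.
; BeginPlay triggers DamagePlayer, which prints the result of Attackplayerimp in two on-screen messages, with each evaluation subtracting Damage from HealthPoint.
; Attackplayer duplicates that subtract-and-return logic but sits in an unconnected part of the event graph and never runs.
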(event Custom|DamagePlayer
  (bind _damage (Variables|Default|GetDamage))
  (bind _newparam (CallFunction|Attackplayerimp _damage))
  (Development|PrintString (Utilities|String|ToString(Integer) _newparam) true true "(R=0.000000,G=0.660000,B=1.000000,A=1.000000)" 2e+01)
  (Development|PrintString (Utilities|String|ToString(Integer) _newparam) true true "(R=0.000000,G=0.660000,B=1.000000,A=1.000000)" 2e+01))

(event EventBeginPlay
  (CallFunction|DamagePlayer))

(fn ConstructionScript)

(fn Attackplayer
  (params (Damage :type Integer))
  (bind _output_get (Variables|Default|SetHealthPoint (- (Variables|Default|GetHealthPoint) Damage)))
  (return _output_get))

(fn Attackplayerimp
  (params (Damage :type Integer))
  (bind _output_get (Variables|Default|SetHealthPoint (- (Variables|Default|GetHealthPoint) Damage)))
  (return _output_get))